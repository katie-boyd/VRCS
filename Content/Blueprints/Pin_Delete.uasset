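; Delete pin actor that removes circuit parts it touches in a VR circuit-building game.
; Overlaps on the actor or its pin models call GetComponentToDelete, which tries a cast for each part type, from resistors and sources to test equipment and ground.
; A match is removed from the VRPawn's ComponentList and destroyed.
; Wires skip the list and have their cable and actor destroyed directly.
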(event OnComponentBeginOverlap(DeletePinModel)
  (params (OverlappedComponent :type Primitive%20Component%20Object%20Reference) (OtherActor :type Actor%20Object%20Reference) (OtherComp :type Primitive%20Component%20Object%20Reference) (OtherBodyIndex :type Integer) (bFromSweep :type Boolean) (SweepResult :type Hit%20Result%20Structure%20%28by%20ref%29))
  (CallFunction|GetComponenttoDelete OtherComp (stale Collision|EventActorBeginOverlap OtherActor)))

(event OnComponentBeginOverlap(PinBottomModel)
  (params (OverlappedComponent :type Primitive%20Component%20Object%20Reference) (OtherActor :type Actor%20Object%20Reference) (OtherComp :type Primitive%20Component%20Object%20Reference) (OtherBodyIndex :type Integer) (bFromSweep :type Boolean) (SweepResult :type Hit%20Result%20Structure%20%28by%20ref%29))
  (CallFunction|GetComponenttoDelete (stale OnComponentBeginOverlap(DeletePinModel) OtherComp) (stale Collision|EventActorBeginOverlap OtherActor)))

(event OnComponentHit(Pin_Sphere)
  (params (HitComponent :type Primitive%20Component%20Object%20Reference) (OtherActor :type Actor%20Object%20Reference) (OtherComp :type Primitive%20Component%20Object%20Reference) (NormalImpulse :type Vector :default "0, 0, 0") (Hit :type Hit%20Result%20Structure%20%28by%20ref%29)))

(event OnComponentHit(DeletePinModel)
  (params (HitComponent :type Primitive%20Component%20Object%20Reference) (OtherActor :type Actor%20Object%20Reference) (OtherComp :type Primitive%20Component%20Object%20Reference) (NormalImpulse :type Vector :default "0, 0, 0") (Hit :type Hit%20Result%20Structure%20%28by%20ref%29)))

(event EventBeginPlay)

(event Collision|EventActorBeginOverlap
  (params (OtherActor :type Actor%20Object%20Reference))
  (CallFunction|GetComponenttoDelete (stale OnComponentBeginOverlap(DeletePinModel) OtherComp) OtherActor))

(event EventTick
  (params (DeltaSeconds :type Float%20%28single-precision%29)))

(fn ConstructionScript)

(fn GetComponenttoDelete
  (params (CollidedComponent :type Primitive%20Component%20Object%20Reference) (CollidedActor :type Actor%20Object%20Reference))
  (Utilities|FlowControl|Sequence
    (:then_0
      (bind _asvrpawn (Utilities|Casting|CastToVRPawn (Game|Player|GetPlayerPawn 0))))
    (:then_1
      ;[1 1 1] Resistor
      (bind _asresistor_new (Utilities|Casting|CastToResistor_new CollidedActor))
      (CallFunction|DeleteComponentinArray CollidedActor (Variables|/Game/Blueprints/Components/VRPawn.VRPawn_C|GetComponentList _asvrpawn))
      (Actor|DestroyActor _asresistor_new))
    (:then_2
      ;[1 1 1] Capacitor
      (bind _ascapacitor_new (Utilities|Casting|CastToCapacitor_new CollidedActor))
      (CallFunction|DeleteComponentinArray CollidedActor (Variables|/Game/Blueprints/Components/VRPawn.VRPawn_C|GetComponentList _asvrpawn))
      (Actor|DestroyActor _ascapacitor_new))
    (:then_3
      ;[1 1 1] Inductor
      (bind _asinductor_new (Utilities|Casting|CastToInductor_new CollidedActor))
      (CallFunction|DeleteComponentinArray CollidedActor (Variables|/Game/Blueprints/Components/VRPawn.VRPawn_C|GetComponentList _asvrpawn))
      (Actor|DestroyActor _asinductor_new))
    (:then_4
      ;[1 1 1] Switch
      (bind _asswitch_new (Utilities|Casting|CastToSwitch_new CollidedActor))
      (CallFunction|DeleteComponentinArray CollidedActor (Variables|/Game/Blueprints/Components/VRPawn.VRPawn_C|GetComponentList _asvrpawn))
      (Actor|DestroyActor _asswitch_new))
    (:then_5
      ;[1 1 1] LED
      (bind _asled_new (Utilities|Casting|CastToLED_new CollidedActor))
      (CallFunction|DeleteComponentinArray CollidedActor (Variables|/Game/Blueprints/Components/VRPawn.VRPawn_C|GetComponentList _asvrpawn))
      (Actor|DestroyActor _asled_new))
    (:then_6
      ;[1 1 1] Diode
      (bind _asdiode_new (Utilities|Casting|CastToDiode_new CollidedActor))
      (CallFunction|DeleteComponentinArray CollidedActor (Variables|/Game/Blueprints/Components/VRPawn.VRPawn_C|GetComponentList _asvrpawn))
      (Actor|DestroyActor _asdiode_new))
    (:then_7
      ;[1 1 1] DC
      (bind _asdc_new (Utilities|Casting|CastToDC_new CollidedActor))
      (CallFunction|DeleteComponentinArray CollidedActor (Variables|/Game/Blueprints/Components/VRPawn.VRPawn_C|GetComponentList _asvrpawn))
      (Actor|DestroyActor _asdc_new))
    (:then_8
      ;[1 1 1] AC
      (bind _asac_new (Utilities|Casting|CastToAC_new CollidedActor))
      (CallFunction|DeleteComponentinArray CollidedActor (Variables|/Game/Blueprints/Components/VRPawn.VRPawn_C|GetComponentList _asvrpawn))
      (Actor|DestroyActor _asac_new))
    (:then_9
      ;[1 1 1] test equipment
      (bind _astest_equipment_new (Utilities|Casting|CastToTestEquipment_new CollidedActor))
      (CallFunction|DeleteComponentinArray CollidedActor (Variables|/Game/Blueprints/Components/VRPawn.VRPawn_C|GetComponentList _asvrpawn))
      (Actor|DestroyActor _astest_equipment_new))
    (:then_10
      ;[1 1 1] Ground
      (bind _asground_new (Utilities|Casting|CastToGround_new CollidedActor))
      (CallFunction|DeleteComponentinArray CollidedActor (Variables|/Game/Blueprints/Components/VRPawn.VRPawn_C|GetComponentList _asvrpawn))
      (Actor|DestroyActor _asground_new))
    (:then_11
      ;[1 1 1] Wires
      (bind _aswire (Utilities|Casting|CastTowire CollidedActor)
        (:then
          (Components|DestroyComponent (Variables|/Game/Blueprints/wire.wire_C|GetCable _aswire))
          (Actor|DestroyActor _aswire))
        (:CastFailed
          (Development|PrintString "Hello"))))))

(fn DeleteComponentinArray
  (params (DeletedComponent :type Actor%20Object%20Reference) (ComponentList :type Array%20of%20Actor%20Object%20References))
  (Utilities|Array|RemoveIndex ComponentList (Utilities|Array|FindItem ComponentList DeletedComponent))
  (return))