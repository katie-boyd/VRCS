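; An actor Blueprint for "Okkin", an object in a VR game that can detect and move to the player's left controller.
; Body_collision overlaps set OkkinContCollide when the other component is the VRPawn's Lcollision, printing the result for debugging.
; BringOkkin sweeps the actor to the pawn's ControllerL location; nothing in this Blueprint calls it or reads the flag.
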(event OnComponentBeginOverlap(body_collision)
  (params (OverlappedComponent :type Primitive%20Component%20Object%20Reference) (OtherActor :type Actor%20Object%20Reference) (OtherComp :type Primitive%20Component%20Object%20Reference) (OtherBodyIndex :type Integer) (bFromSweep :type Boolean) (SweepResult :type Hit%20Result%20Structure%20%28by%20ref%29))
  (bind _asvrpawn (Utilities|Casting|CastToVRPawn (Game|Player|GetPlayerPawn 0)))
  (bind _output_get (Variables|Default|Setokkin_cont_collide (== OtherComp (Variables|/Game/Blueprints/Components/VRPawn.VRPawn_C|GetLcollision _asvrpawn))))
  (if _output_get
    (Development|PrintString "true")
    (else
      (Development|PrintString "false"))))

(event EventBeginPlay)

(event Collision|EventActorBeginOverlap
  (params (OtherActor :type Actor%20Object%20Reference)))

(event EventTick
  (params (DeltaSeconds :type Float%20%28single-precision%29)))

(fn ConstructionScript)

(fn BringOkkin
  (bind _asvrpawn (Utilities|Casting|CastToVRPawn (Game|Player|GetPlayerPawn 0)))
  (Transformation|SetActorLocation (.Location (Math|Transform|BreakTransform (Transformation|GetWorldTransform (Variables|/Game/Blueprints/Components/VRPawn.VRPawn_C|GetController_L _asvrpawn)))) true false))