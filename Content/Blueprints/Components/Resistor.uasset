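; Resistor actor for a VR game, currently a prototype that tests whether the player's hand touches it.
; When Resistorcube begins an overlap, it compares the other component to the VR pawn's Lcollision and prints a debug string for match or mismatch.
; The trace activate, hit, leave and move functions and Sendsphereprimcompoent are stubs that only return false.
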(event OnComponentBeginOverlap(resistorcube)
  (params (OverlappedComponent :type Primitive%20Component%20Object%20Reference) (OtherActor :type Actor%20Object%20Reference) (OtherComp :type Primitive%20Component%20Object%20Reference) (OtherBodyIndex :type Integer) (bFromSweep :type Boolean) (SweepResult :type Hit%20Result%20Structure%20%28by%20ref%29))
  (bind _asvrpawn (Utilities|Casting|CastToVRPawn (Game|Player|GetPlayerPawn 0)))
  (bind _output_get (Variables|Default|Sethascolldided (== (Variables|/Game/Blueprints/Components/VRPawn.VRPawn_C|GetLcollision _asvrpawn) OtherComp)))
  (if _output_get
    (Development|PrintString "yar")
    (else
      (Development|PrintString "nar"))))

(event EventBeginPlay)

(event Collision|EventActorBeginOverlap
  (params (OtherActor :type Actor%20Object%20Reference)))

(event EventTick
  (params (DeltaSeconds :type Float%20%28single-precision%29)))

(fn ConstructionScript)

(fn NewFunction0)

(fn Sendsphereprimcompoent
  (params (inresistorcube :type Boolean))
  (return false))

(fn TraceActivateDown
  (params (Hit :type Hit%20Result%20Structure%20%28by%20ref%29) (Pawn :type Pawn%20Object%20Reference%20%28by%20ref%29))
  (return false))

(fn TraceActivateUp
  (params (Hit :type Hit%20Result%20Structure%20%28by%20ref%29) (Pawn :type Pawn%20Object%20Reference%20%28by%20ref%29))
  (return false))

(fn TraceHitComponent
  (params (Hit :type Hit%20Result%20Structure) (Component :type Primitive%20Component%20Object%20Reference))
  (return false))

(fn TraceHitObject
  (params (Hit :type Hit%20Result%20Structure))
  (return false))

(fn TraceLeaveComponent
  (params (Hit :type Hit%20Result%20Structure) (Component :type Primitive%20Component%20Object%20Reference))
  (return false))

(fn TraceLeaveObject
  (params (Hit :type Hit%20Result%20Structure))
  (return false))

(fn TraceMove
  (params (Hit :type Hit%20Result%20Structure%20%28by%20ref%29))
  (return false))