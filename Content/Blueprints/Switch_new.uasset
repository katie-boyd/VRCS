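; VR toggle switch that the player flips with the left hand.
; When the VRPawn's left collision overlaps SwitchThrow while SwitchLPressed is set, it toggles the On/Off State, rotates the throw and clears the flag.
; Moveswitch sets the roll with a single high-speed FInterpTo call per toggle, with no per-tick animation.
; Failed pawn casts and left-hand overlaps without a press print a debug string.
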(event OnComponentBeginOverlap(SwitchThrow)
  (params (OverlappedComponent :type Primitive%20Component%20Object%20Reference) (OtherActor :type Actor%20Object%20Reference) (OtherComp :type Primitive%20Component%20Object%20Reference) (OtherBodyIndex :type Integer) (bFromSweep :type Boolean) (SweepResult :type Hit%20Result%20Structure%20%28by%20ref%29))
  (bind _asvrpawn (Utilities|Casting|CastToVRPawn (Game|Player|GetPlayerPawn 0))
    (:then
      (if (== (Variables|/Game/Blueprints/Components/VRPawn.VRPawn_C|GetLcollision _asvrpawn) OtherComp)
        (if (Variables|/Game/Blueprints/Components/VRPawn.VRPawn_C|GetswitchLPressed _asvrpawn)
          (switch Utilities|FlowControl|Switch|SwitchonESwitchStates (Variables|Default|GetState)
            (:NewEnumerator0
              (Variables|Default|SetState "NewEnumerator1")
              (CallFunction|Moveswitch 0.0))
            (:NewEnumerator1
              (Variables|Default|SetState "NewEnumerator0")
              (CallFunction|Moveswitch 9e+01)))
          (Variables|/Game/Blueprints/Components/VRPawn.VRPawn_C|SetswitchLPressed _asvrpawn false)
          (else
            (Development|PrintString "Hello")))))
    (:CastFailed
      (Development|PrintString "Hello"))))

(event Custom|moveswitch
  (params (RotationToSet :type Float%20%28single-precision%29))
  (Transformation|SetRelativeRotation (Variables|Default|GetSwitchThrow) (Math|Rotator|MakeRotator (Math|Interpolation|FInterpTo (.Roll (Math|Rotator|BreakRotator (Variables|/Script/Engine.SceneComponent|GetRelativeRotation (Variables|Default|GetSwitchThrow)))) RotationToSet (Utilities|Time|GetWorldDeltaSeconds) 1e+02) 0.0 0.0) false false))

(event EventBeginPlay)

(event Collision|EventActorBeginOverlap
  (params (OtherActor :type Actor%20Object%20Reference)))

(event EventTick
  (params (DeltaSeconds :type Float%20%28single-precision%29)))

(fn ConstructionScript)